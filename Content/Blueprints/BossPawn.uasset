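; Boss enemy pawn that takes damage, tracks its health and destroys itself when health runs out.
; AnyDamage plays a hit montage, ignoring further hits until it completes, and passes the DamageType's processed value to UpdateHealth.
; UpdateHealth adds that value, clamps between zero and base health, and fires NoHealthLeft at zero.
; ShowWeaponEnemy, uncalled here, spawns an unattached Shovel for Florist or hides the actor for Student and Mage.
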(event Custom|NoHealthLeft
  ;[1 1 1] Die
  (Development|PrintString "Enemy died!")
  (Actor|DestroyActor))

(event Collision|EventActorBeginOverlap
  (params (OtherActor :type Actor%20Object%20Reference)))

(event EventTick
  (params (DeltaSeconds :type Float%20%28single-precision%29)))

(event EventBeginPlay)

(event Game|Damage|EventAnyDamage
  (params (Damage :type Float%20%28single-precision%29) (DamageType :type Damage%20Type%20Object%20Reference) (InstigatedBy :type Controller%20Object%20Reference) (DamageCauser :type Actor%20Object%20Reference))
  ;[1 1 1] On receving damage
  (if (not (Variables|Default|GetReceivingDamage?))
    (Variables|Default|SetReceivingDamage? true)
    (Animation|Montage|PlayMontage (Variables|Character|GetMesh) "/Game/anim/HitMontage.HitMontage"
      (:then
        (bind _output_get (Variables|Default|SetDamageType DamageType))
        (bind _damageout (Class|ProcessDamage|ProcessDamage(Message) _output_get Damage))
        (bind _result (Math|Float|NegateFloat _damageout)
          (:%20%20
            (Development|PrintString (Utilities|String|ToString(Float) _result))
            (CallFunction|UpdateHealth _result))))
      (:OnCompleted
        (Variables|Default|SetReceivingDamage? false)))))

(fn ConstructionScript)

(fn UpdateHealth
  (params (changeValue :type Float%20%28single-precision%29))
  (if (> (+ changeValue (Variables|Default|GetCurrentEnemyHealth)) (Variables|Default|GetEnemyBaseHealth))
    (Variables|Default|SetCurrentEnemyHealth (Variables|Default|GetEnemyBaseHealth))
    (elif (<= (+ changeValue (Variables|Default|GetCurrentEnemyHealth)) 0.0)
      (Variables|Default|SetCurrentEnemyHealth 0.0)
      (CallFunction|NoHealthLeft)
      (else
        (Variables|Default|SetCurrentEnemyHealth (+ changeValue (Variables|Default|GetCurrentEnemyHealth))))))
  (return (Variables|Default|GetCurrentEnemyHealth)))

(fn ShowWeaponEnemy
  (params (EnemyType :type EnemyTypeEnum%20Enum :default "NewEnumerator0"))
  (switch Utilities|FlowControl|Switch|SwitchonEnemyTypeEnum EnemyType
    (:NewEnumerator0
      (Game|SpawnActorfromClass "/Game/Blueprints/Weapons/Shovel.Shovel_C" (Math|Transform|MakeTransform "0, 0, 0") "Undefined" 0 0))
    (:NewEnumerator1
      (Rendering|SetActorHiddenInGame true :!label _label))
    (:NewEnumerator2
      (goto _label))))