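; Enemy pawn for a side-on game, with EnemyType (Florist, Student, Mage) selecting health, mesh, animation, weapon and attacks.
; Tick locks it to Y=0 and turns it toward the player, pinning it and switching its collision channel while the player dashes.
; Sighting the player triggers type-specific chasing or retreating, then montage attacks; ThrowStuff spawns random projectiles.
; Damage plays a hit montage and updates health; death drops a type-matched SoulShard.
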(event OnSeePawn(PawnSensing)
  (params (Pawn :type Pawn%20Object%20Reference))
  (bind _returnvalue (Transformation|GetActorLocation))
  (bind _returnvalue_2 (Game|Player|GetPlayerPawn 0))
  (bind _returnvalue_3 (Transformation|GetActorLocation))
  (bind _self self)
  (bind _asmain_character_pawn (Utilities|Casting|CastToMainCharacterPawn (Game|Player|GetPlayerPawn 0)))
  (if (not (Variables|/Game/Blueprints/MainCharacterPawn.MainCharacterPawn_C|GetNotAllowedToMove? _asmain_character_pawn))
    (switch Utilities|FlowControl|Switch|SwitchonEnemyTypeEnum (Variables|Default|GetEnemyType)
      (:NewEnumerator0
        ;[1 1 1] GrayBeard
        (AI|AIMoveTo self "0, 0, 0" _returnvalue_2 5.0 false
          (:OnSuccess
            (Variables|Default|SetTargetRotation (Math|Conversions|RotationFromXVector (Math|Transform|InverseTransformLocation (Transformation|GetActorTransform) (Transformation|GetActorLocation _returnvalue_2))))
            (CallFunction|DoNormalAttack))))
      (:NewEnumerator1
        ;[1 1 1] Student
        (if (not (Variables|Default|GetPerformingAttack?))
          (if (> 4.5e+02 (Math|Vector|VectorLength (- (Transformation|GetActorLocation Pawn) (Transformation|GetActorLocation))))
            (if (Math|Float|NearlyEqual(Float) (.yaw (Transformation|GetActorRotation)) 1.8e+02 2.0)
              (AI|AIMoveTo _self (Math|Vector|MakeVector (+ (.x _returnvalue_3) 4.5e+02) 0.0 (.z _returnvalue_3)) 0 5.0 false
                (:OnSuccess
                  _)
                (:OnFail
                  _))
              (else
                (AI|AIMoveTo _self (Math|Vector|MakeVector (+ (.x _returnvalue_3) -4.5e+02) 0.0 (.z _returnvalue_3)) 0 5.0 false
                  (:OnSuccess
                    _)
                  (:OnFail
                    _)))))
          (CallFunction|DoNormalAttack)))
      (:NewEnumerator2
        ;[1 1 1] Magician
        (if (not (Variables|Default|GetPerformingAttack?))
          (if (> 1.5e+02 (Math|Vector|VectorLength (- (Transformation|GetActorLocation Pawn) (Transformation|GetActorLocation))))
            (if (Math|Float|NearlyEqual(Float) (.yaw (Transformation|GetActorRotation)) 1.8e+02 2.0)
              (AI|AIMoveTo 0 (Math|Vector|MakeVector (+ (.x _returnvalue) 1.5e+02) 0.0 (.z _returnvalue)) 0 5.0 false
                (:OnSuccess
                  _)
                (:OnFail
                  _))
              (else
                (AI|AIMoveTo self (Math|Vector|MakeVector (+ (.x _returnvalue) -3e+02) 0.0 (.z _returnvalue)) 0 5.0 false
                  (:OnSuccess
                    _)
                  (:OnFail
                    _))))
            (CallFunction|DoNormalAttack)
            (elif (> (Math|Vector|VectorLength (- (Transformation|GetActorLocation) (Transformation|GetActorLocation))) 3e+02)
              (AI|AIMoveTo self "0, 0, 0" (Game|Player|GetPlayerPawn 0) 3e+02 false
                (:OnSuccess
                  (CallFunction|DoNormalAttack)))
              (else
                (CallFunction|DoNormalAttack)))))))))

(event Custom|NoHealthLeft
  ;[1 1 1] Die
  (Actor|DestroyActor (Variables|Default|GetShovel))
  (if (not (Variables|Default|GetDied))
    (bind _returnvalue (Game|SpawnActorfromClass "/Game/GameplayElements/SoulShard.SoulShard_C" (Math|Transform|MakeTransform (Transformation|GetActorLocation)) "Undefined" 0 0))
    (Variables|/Game/GameplayElements/SoulShard.SoulShard_C|SetSoulShardType _returnvalue (Utilities|Select :Index (Variables|Default|GetEnemyType) :NewEnumerator0 "NewEnumerator1" :NewEnumerator1 "NewEnumerator2" :NewEnumerator2 "NewEnumerator3"))
    (Default|UpdateColour _returnvalue)
    (Development|SetHiddeninGame (Variables|Character|GetMesh) true false)
    (Collision|SetCollisionEnabled (Variables|Collision|GetCapsuleComponent) "NoCollision")
    (Components|Activation|Activate (Variables|Default|GetVFX) true)
    (Actor|DestroyActor)))

(event Custom|DoNormalAttack
  (bind _mesh (Variables|Character|GetMesh))
  ;[1 1 1] Do normal attack
  (if (not (Variables|Default|GetReceivingDamage?))
    (if (not (Variables|Default|GetPerformingAttack?))
      (switch Utilities|FlowControl|Switch|SwitchonEnemyTypeEnum (Variables|Default|GetEnemyType)
        (:NewEnumerator0
          (Animation|Montage|PlayMontage _mesh "/Game/anim/shovel/ShovelMontage.ShovelMontage"
            (:then
              (Variables|Default|SetPerformingAttack? true :!label _label))
            (:OnCompleted
              (Variables|Default|SetPerformingAttack? false :!label _label_2))
            (:OnInterrupted
              (goto _label_2))))
        (:NewEnumerator1
          (Animation|Montage|PlayMontage _mesh "/Game/anim/girl/ThrowMontage.ThrowMontage"
            (:then
              (goto _label))
            (:OnCompleted
              (goto _label_2))
            (:OnInterrupted
              (goto _label_2))))
        (:NewEnumerator2
          (Animation|Montage|PlayMontage _mesh "/Game/anim/magic/Magic1Montage.Magic1Montage"
            (:then
              (goto _label))
            (:OnCompleted
              (goto _label_2))
            (:OnInterrupted
              (goto _label_2))))))))

(event Custom|DoSpecialAttack
  (bind _mesh (Variables|Character|GetMesh))
  ;[1 1 1] Do special attack
  (switch Utilities|FlowControl|Switch|SwitchonEnemyTypeEnum (Variables|Default|GetEnemyType)
    (:NewEnumerator0
      (Animation|Montage|PlayMontage _mesh "/Game/anim/shovel/ShovelSpecialMontage.ShovelSpecialMontage"
        (:then
          (Variables|Default|SetPerformingAttack? true :!label _label))
        (:OnCompleted
          (Variables|Default|SetPerformingAttack? false :!label _label_2))
        (:OnInterrupted
          (goto _label_2))))
    (:NewEnumerator1
      (Animation|Montage|PlayMontage _mesh "/Game/anim/girl/PowerfulThrowMontage.PowerfulThrowMontage"
        (:then
          (goto _label))
        (:OnCompleted
          (goto _label_2))
        (:OnInterrupted
          (goto _label_2))))
    (:NewEnumerator2
      (Animation|Montage|PlayMontage _mesh "/Game/anim/magic/Magic2Montage.Magic2Montage"
        (:then
          (goto _label))
        (:OnCompleted
          (goto _label_2))
        (:OnInterrupted
          (goto _label_2))))))

(event Custom|updateSoul
  (bind _enemytype (Variables|Default|GetEnemyType))
  (bind _mesh (Variables|Character|GetMesh))
  ;[1 1 1] Update soul
  (Class|SkinnedMeshComponent|SetSkeletalMesh _mesh (Utilities|Select :Index _enemytype :NewEnumerator0 "/Game/char/graybeard/graybeard.graybeard" :NewEnumerator1 "/Game/char/Sayaka/sayaka.sayaka" :NewEnumerator2 0) true)
  (Class|SkeletalMeshComponent|SetAnimClass _mesh (Utilities|Select :Index _enemytype :NewEnumerator0 "/Game/anim/shovel/ShovelAnimBP.ShovelAnimBP_C" :NewEnumerator1 "/Game/anim/girl/GirlAnimBP.GirlAnimBP_C" :NewEnumerator2 0))
  (CallFunction|ShowWeaponEnemy (Variables|Default|GetEnemyType)))

(event EventThrowStuff
  (params (NormalAttack? :type Boolean) (Transform :type Transform))
  ;[1 1 1] Throw projectile
  (switch int (Math|Random|RandomIntegerinRange 0 3)
    (:0
      (Variables|Default|SetProjectileToLaunch "/Game/Blueprints/Projectiles/ProjectileBook.ProjectileBook_C"))
    (:1
      (Variables|Default|SetProjectileToLaunch "/Game/Blueprints/Projectiles/ProjectileEraser.ProjectileEraser_C"))
    (:2
      (Variables|Default|SetProjectileToLaunch "/Game/Blueprints/Projectiles/ProjectilePen.ProjectilePen_C"))
    (:3
      (Variables|Default|SetProjectileToLaunch "/Game/Blueprints/Projectiles/ProjectileRuler.ProjectileRuler_C")))
  (bind _returnvalue (Game|SpawnActorfromClass (Variables|Default|GetProjectileToLaunch) (Math|Transform|MakeTransform (.location Transform) (Math|Rotator|MakeRotator (.roll (.rotation Transform)) (.pitch (Variables|Default|GetTargetRotation)) (.yaw (.rotation Transform))) (.scale Transform)) "Undefined" 0 0))
  (bind _asprojectile (Utilities|Casting|CastToProjectile _returnvalue))
  (if (not NormalAttack?)
    (Variables|/Game/Blueprints/Projectiles/Projectile.Projectile_C|SetthrowingActor _asprojectile self)
    (Game|Components|ProjectileMovement|SetVelocityinLocalSpace (Variables|/Game/Blueprints/Projectiles/Projectile.Projectile_C|GetProjectileMovement _asprojectile) (* (Variables|/Script/Engine.MovementComponent|GetVelocity (Variables|/Game/Blueprints/Projectiles/Projectile.Projectile_C|GetProjectileMovement _asprojectile)) 3.0))))

(event EventTick
  (params (DeltaSeconds :type Float%20%28single-precision%29))
  (bind _returnvalue (Transformation|GetActorLocation))
  (bind _capsulecomponent (Variables|Collision|GetCapsuleComponent))
  ;[1 1 1] BaseBehaviour
  (bind _asmain_character_pawn (Utilities|Casting|CastToMainCharacterPawn (Game|Player|GetPlayerPawn 0)))
  (if (Variables|/Game/Blueprints/MainCharacterPawn.MainCharacterPawn_C|GetIsDashing? _asmain_character_pawn)
    (Utilities|FlowControl|Sequence
      (:then_0
        (Utilities|FlowControl|DoOnce false :!label _label
          (:Completed
            (Variables|Default|SetLastLocation%20 (Transformation|GetActorLocation)))))
      (:then_1
        (Collision|SetCollisionObjectType _capsulecomponent "ECC_GameTraceChannel2")
        (Transformation|SetActorLocation (Variables|Default|GetLastLocation%20) false true)
        (if (not (Variables|/Game/Blueprints/MainCharacterPawn.MainCharacterPawn_C|GetNotAllowedToMove? _asmain_character_pawn)) :!label _label_2
          (Transformation|SetActorLocation (Math|Vector|MakeVector (.x _returnvalue) 0.0 (.z _returnvalue)) false true)
          (bind _asmain_character_pawn_2 (Utilities|Casting|CastToMainCharacterPawn (Game|Player|GetPlayerPawn 0)))
          (if (> (.x (Transformation|GetActorLocation _asmain_character_pawn_2)) (.x (Transformation|GetActorLocation)))
            (Transformation|SetActorRotation "0, 0, 0")
            (else
              (Transformation|SetActorRotation "0,180.000000, 0"))))))
    (else
      (Utilities|FlowControl|Sequence
        (:then_0
          (goto _label Reset))
        (:then_1
          (Collision|SetCollisionObjectType _capsulecomponent "ECC_Pawn")
          (goto _label_2))))))

(event EventBeginPlay
  (bind _mesh (Variables|Character|GetMesh))
  (bind _enemytype (Variables|Default|GetEnemyType))
  ;[1 1 1] Set up mesh and base variables
  (switch Utilities|FlowControl|Switch|SwitchonEnemyTypeEnum (Variables|Default|GetEnemyType)
    (:NewEnumerator0
      (Variables|Default|SetEnemyBaseHealth 4e+01))
    (:NewEnumerator1
      (Variables|Default|SetEnemyBaseHealth 2e+01))
    (:NewEnumerator2
      (Variables|Default|SetEnemyBaseHealth 1e+02)))
  (Variables|Default|SetCurrentEnemyHealth (Variables|Default|GetEnemyBaseHealth))
  (Class|SkinnedMeshComponent|SetSkeletalMesh _mesh (Utilities|Select :Index _enemytype :NewEnumerator0 "/Game/char/graybeard/graybeard.graybeard" :NewEnumerator1 "/Game/char/Sayaka/sayaka.sayaka" :NewEnumerator2 0) true)
  (Class|SkeletalMeshComponent|SetAnimClass _mesh (Utilities|Select :Index _enemytype :NewEnumerator0 "/Game/anim/shovel/ShovelAnimBP.ShovelAnimBP_C" :NewEnumerator1 "/Game/anim/girl/GirlAnimBP.GirlAnimBP_C" :NewEnumerator2 0))
  (CallFunction|ShowWeaponEnemy (Variables|Default|GetEnemyType)))

(event Game|Damage|EventAnyDamage
  (params (Damage :type Float%20%28single-precision%29) (DamageType :type Damage%20Type%20Object%20Reference) (InstigatedBy :type Controller%20Object%20Reference) (DamageCauser :type Actor%20Object%20Reference))
  ;[1 1 1] On receving damage
  (if (Variables|Default|GetReceivingDamage?)
    _
    (else
      (Variables|Default|SetReceivingDamage? true)))
  (Animation|Montage|PlayMontage (Variables|Character|GetMesh) "/Game/anim/HitMontage.HitMontage"
    (:then
      (bind _output_get (Variables|Default|SetDamageType DamageType))
      (bind _damageout (Class|ProcessDamage|ProcessDamage(Message) _output_get Damage))
      (bind _result (Math|Float|NegateFloat _damageout)
        (:%20%20
          (Development|PrintString (Utilities|String|ToString(Float) _result))
          (Utilities|FlowControl|Delay 0.1)
          (CallFunction|UpdateHealth _result))))
    (:OnCompleted
      (Variables|Default|SetReceivingDamage? false :!label _label))
    (:OnBlendOut
      (goto _label))
    (:OnInterrupted
      (goto _label))))

(fn ConstructionScript)

(fn UpdateHealth
  (params (changeValue :type Float%20%28single-precision%29))
  (if (> (+ changeValue (Variables|Default|GetCurrentEnemyHealth)) (Variables|Default|GetEnemyBaseHealth))
    (Variables|Default|SetCurrentEnemyHealth (Variables|Default|GetEnemyBaseHealth))
    (elif (<= (+ changeValue (Variables|Default|GetCurrentEnemyHealth)) 0.0)
      (Variables|Default|SetCurrentEnemyHealth 0.0)
      (CallFunction|NoHealthLeft)
      (else
        (Variables|Default|SetCurrentEnemyHealth (+ changeValue (Variables|Default|GetCurrentEnemyHealth))))))
  (return (Variables|Default|GetCurrentEnemyHealth)))

(fn ApplyDamageMultiplier
  (params (Damage :type Float%20%28single-precision%29) (Multiplier :type Float%20%28single-precision%29))
  (return (* Damage Multiplier)))

(fn ShowWeaponEnemy
  (params (EnemyType :type EnemyTypeEnum%20Enum :default "NewEnumerator0"))
  (switch Utilities|FlowControl|Switch|SwitchonEnemyTypeEnum EnemyType
    (:NewEnumerator0
      (bind _returnvalue (Game|SpawnActorfromClass "/Game/Blueprints/Weapons/Shovel.Shovel_C" (Math|Transform|MakeTransform "0, 0, 0") "Undefined" 0 0))
      (bind _output_get (Variables|Default|SetShovel _returnvalue))
      (Transformation|AttachComponentToComponent _output_get (Variables|Character|GetMesh) "Hand_r" "KeepRelative" "KeepRelative" "KeepRelative" true))
    (:NewEnumerator1
      (Rendering|SetActorHiddenInGame (Variables|Default|GetShovel) true :!label _label))
    (:NewEnumerator2
      (goto _label))))