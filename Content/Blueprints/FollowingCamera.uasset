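; FollowingCamera is a side-view camera actor that follows the main character in X and Z, using restriction sizes and height offsets from BaseGameMode.
; Tick clamps it within a box around the player, with the vertical offset switching when looking down.
; RecenterCamera timeline-blends back to the player and can be aborted.
; Until OnPlayer is set, it holds a high position; GoToPlayerLocation animates its height, then enables following, player movement and HUD.
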(event Custom|RecenterCamera
  ;[1 1 1] RecenterCamera
  (if (Variables|Default|GetOnPlayer?)
    (Variables|Default|SetOldCameraPosition (Transformation|GetActorLocation))
    (bind _blendamount (Timeline|ReCenterCam PlayFromStart)
      (:Update
        (bind _asmain_character_pawn (Utilities|Casting|CastToMainCharacterPawn (Game|GetPlayerCharacter 0)))
        (Variables|Default|SetDesiredCameraPosition (Math|Vector|MakeVector (.x (Transformation|GetWorldLocation (Variables|/Script/Engine.Character|GetCapsuleComponent _asmain_character_pawn))) (.y (Transformation|GetActorLocation)) (+ (.z (Transformation|GetWorldLocation (Variables|/Script/Engine.Character|GetCapsuleComponent _asmain_character_pawn))) (CallFunction|FindOffset))))
        (Transformation|SetActorLocation (+ (* (Variables|Default|GetDesiredCameraPosition) _blendamount) (* (Variables|Default|GetOldCameraPosition) (+ (* _blendamount -1.0) 1.0))) false false)))))

(event Custom|AbortRecenter
  ;[1 1 1] RecenterCamera
  (bind _blendamount (Timeline|ReCenterCam Stop)
    (:Update
      (bind _asmain_character_pawn (Utilities|Casting|CastToMainCharacterPawn (Game|GetPlayerCharacter 0)))
      (Variables|Default|SetDesiredCameraPosition (Math|Vector|MakeVector (.x (Transformation|GetWorldLocation (Variables|/Script/Engine.Character|GetCapsuleComponent _asmain_character_pawn))) (.y (Transformation|GetActorLocation)) (+ (.z (Transformation|GetWorldLocation (Variables|/Script/Engine.Character|GetCapsuleComponent _asmain_character_pawn))) (CallFunction|FindOffset))))
      (Transformation|SetActorLocation (+ (* (Variables|Default|GetDesiredCameraPosition) _blendamount) (* (Variables|Default|GetOldCameraPosition) (+ (* _blendamount -1.0) 1.0))) false false))))

(event Custom|GoToPlayerLocation
  (bind _newtrack_0 (Timeline|MoveCameraTimeline PlayFromStart)
    (:Update
      (Transformation|SetActorLocation (Math|Vector|MakeVector 0.0 7e+02 _newtrack_0) true false))
    (:Finished
      (Variables|Default|SetOnPlayer? true)
      (bind _asmain_character_pawn (Utilities|Casting|CastToMainCharacterPawn (Game|Player|GetPlayerPawn 0)))
      (Variables|/Game/Blueprints/MainCharacterPawn.MainCharacterPawn_C|SetNotAllowedToMove? _asmain_character_pawn false)
      (Widget|SetVisibility (Variables|/Game/Blueprints/MainCharacterPawn.MainCharacterPawn_C|GetSoulShardsHUD _asmain_character_pawn) "Visible"))))

(event EventBeginPlay
  (bind _asbase_game_mode (Utilities|Casting|CastToBaseGameMode (Game|GetGameMode)))
  (Variables|Default|SetRestrictionWidth (Variables|/Game/Blueprints/BaseGameMode.BaseGameMode_C|GetPlayerRestrictionWidth _asbase_game_mode))
  (Variables|Default|SetLookDownZoffset (Variables|/Game/Blueprints/BaseGameMode.BaseGameMode_C|GetLookDownCameraZoffset _asbase_game_mode))
  (Variables|Default|SetRestrictionHeight (Variables|/Game/Blueprints/BaseGameMode.BaseGameMode_C|GetPlayerRestrictionHeight _asbase_game_mode))
  (Variables|Default|SetZoffset (Variables|/Game/Blueprints/BaseGameMode.BaseGameMode_C|GetCameraZoffset _asbase_game_mode))
  (CallFunction|SetInitialCameraPosition))

(event EventTick
  (params (DeltaSeconds :type Float%20%28single-precision%29))
  (bind _returnvalue (Transformation|GetActorLocation))
  (bind _restrictionwidth (Variables|Default|GetRestrictionWidth))
  (bind _restrictionheight (Variables|Default|GetRestrictionHeight))
  ;[1 1 1] UpdateCameraPosition
  (if (Variables|Default|GetOnPlayer?)
    (bind _asmain_character_pawn (Utilities|Casting|CastToMainCharacterPawn (Game|GetPlayerCharacter 0)))
    (Transformation|SetActorLocation (Math|Vector|MakeVector (Math|Float|Clamp(Float) (.x _returnvalue) (- (.x (Transformation|GetWorldLocation (Variables|/Script/Engine.Character|GetCapsuleComponent _asmain_character_pawn))) _restrictionwidth) (+ (.x (Transformation|GetWorldLocation (Variables|/Script/Engine.Character|GetCapsuleComponent _asmain_character_pawn))) _restrictionwidth)) (.y _returnvalue) (Math|Float|Clamp(Float) (.z _returnvalue) (- (+ (.z (Transformation|GetWorldLocation (Variables|/Script/Engine.Character|GetCapsuleComponent _asmain_character_pawn))) (CallFunction|FindOffset)) _restrictionheight) (+ (+ (.z (Transformation|GetWorldLocation (Variables|/Script/Engine.Character|GetCapsuleComponent _asmain_character_pawn))) (CallFunction|FindOffset)) _restrictionheight))) false false)
    (else
      (Transformation|SetActorLocation (Math|Vector|MakeVector 0.0 7e+02 4e+03) false false))))

(fn ConstructionScript)

(fn SetInitialCameraPosition
  (bind _asmain_character_pawn (Utilities|Casting|CastToMainCharacterPawn (Game|GetPlayerCharacter 0)))
  (Transformation|SetActorLocation (Math|Vector|MakeVector (.x (Transformation|GetWorldLocation (Variables|/Script/Engine.Character|GetCapsuleComponent _asmain_character_pawn))) (.y (Transformation|GetActorLocation)) (+ (.z (Transformation|GetWorldLocation (Variables|/Script/Engine.Character|GetCapsuleComponent _asmain_character_pawn))) (Variables|Default|GetZoffset))) false false))

(fn FindOffset
  (bind _asmain_character_pawn (Utilities|Casting|CastToMainCharacterPawn (Game|GetPlayerCharacter 0)))
  (if (Variables|/Game/Blueprints/MainCharacterPawn.MainCharacterPawn_C|GetLookingDown? _asmain_character_pawn)
    (return (Variables|Default|GetLookDownZoffset))
    (else
      (return (Variables|Default|GetZoffset)))))