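; Base game mode that handles level transitions with a screen fade and a saved respawn location.
; LoadLevel saves the spawn location and open-menu flag to the RespawnLocation slot, shows a ChangingLevel widget, then opens the named level once its fade timeline finishes.
; BeginPlay adds the same widget and plays a second timeline in reverse, with both timelines driving CameraFadeIntensity.
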(event Custom|LoadLevel
  (params (LevelName :type Name) (SpawnLoc :type Vector) (OpenMenu :type Boolean))
  (bind _returnvalue (SaveGame|CreateSaveGameObject "/Game/Blueprints/SaveRespawnLocation.SaveRespawnLocation_C"))
  (Variables|/Game/Blueprints/SaveRespawnLocation.SaveRespawnLocation_C|SetRespawnLocation _returnvalue SpawnLoc)
  (Variables|/Game/Blueprints/SaveRespawnLocation.SaveRespawnLocation_C|SetOpenMenu _returnvalue OpenMenu)
  (SaveGame|SaveGametoSlot _returnvalue "RespawnLocation")
  (bind _returnvalue_2 (UserInterface|CreateWidget "/Game/UI/ChangingLevel.ChangingLevel_C"))
  (UserInterface|Viewport|AddtoViewport _returnvalue_2 0)
  (bind _newtrack_0 (Timeline|ScreenFadeTimeline PlayFromStart)
    (:Update
      (Variables|Camera|SetCameraFadeIntensity _newtrack_0))
    (:Finished
      (Game|OpenLevel(byName) LevelName))))

(event EventTick
  (params (DeltaSeconds :type Float%20%28single-precision%29)))

(event EventBeginPlay
  (bind _returnvalue (UserInterface|CreateWidget "/Game/UI/ChangingLevel.ChangingLevel_C"))
  (UserInterface|Viewport|AddtoViewport _returnvalue 0)
  (bind _newtrack_0 (Timeline|Timeline_0 ReverseFromEnd)
    (:Update
      (Variables|Camera|SetCameraFadeIntensity _newtrack_0))))

(fn ConstructionScript)