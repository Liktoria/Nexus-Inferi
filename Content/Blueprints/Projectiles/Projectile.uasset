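; Thrown projectile actor that damages what it hits, using either the normal or special backpack damage type based on the NormalAttack flag.
; Hitbox overlaps wait briefly, print debug names, and skip the thrower by comparing display names before applying damage.
; When projectile movement stops, rotation halts, the sphere switches to physics simulation, and the actor destroys itself after a short delay.
; The BeginPlay check on the thrower's class leads to no action.
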(event OnProjectileStop(ProjectileMovement)
  (params (ImpactResult :type Hit%20Result%20Structure%20%28by%20ref%29))
  (Variables|/Script/Engine.RotatingMovementComponent|SetRotationRate (Variables|Default|GetRotatingMovement) "0, 0, 0")
  (Physics|SetSimulatePhysics (Variables|Default|GetSphere) true)
  (Utilities|FlowControl|Delay 1.0)
  (Actor|DestroyActor))

(event OnComponentBeginOverlap(Hitbox)
  (params (OverlappedComponent :type Primitive%20Component%20Object%20Reference) (OtherActor :type Actor%20Object%20Reference) (OtherComp :type Primitive%20Component%20Object%20Reference) (OtherBodyIndex :type Integer) (bFromSweep :type Boolean) (SweepResult :type Hit%20Result%20Structure%20%28by%20ref%29))
  (bind _returnvalue (Utilities|GetDisplayName OtherActor))
  (bind _throwingactor (Variables|Default|GetthrowingActor))
  (bind _returnvalue_2 (Utilities|GetDisplayName _throwingactor))
  (Utilities|FlowControl|Delay 0.2)
  (Development|PrintString _returnvalue)
  (Development|PrintString _returnvalue_2)
  (if (not (Utilities|Enum|Equal(Enum) _returnvalue _returnvalue_2))
    (if (Variables|Default|GetnormalAttack?)
      (Game|Damage|ApplyDamage OtherActor 1.0 0 0 "/Game/DamageTypes/BackpackNormal_DT.BackpackNormal_DT_C")
      (else
        (Game|Damage|ApplyDamage OtherActor 1.0 0 0 "/Game/DamageTypes/BackpackSpecial_DT.BackpackSpecial_DT_C")))))

(event EventBeginPlay
  (if (== (Utilities|GetClass (Variables|Default|GetthrowingActor)) (Variables|Default|GetplayerPawn))
    _))

(event Collision|EventActorBeginOverlap
  (params (OtherActor :type Actor%20Object%20Reference)))

(event EventTick
  (params (DeltaSeconds :type Float%20%28single-precision%29)))

(fn ConstructionScript)