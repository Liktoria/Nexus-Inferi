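; Trigger actor that spawns enemies the first time the main character pawn overlaps it.
; A DoOnce gate leads to an AI spawn at Point1, with the pawn class selected by Enemy1; Mage has no class, so it spawns nothing.
; A valid class also spawns a generic EnemyPawn at Point2.
; Logic to set the first enemy's type and update its soul is disconnected.
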(event EventBeginPlay)

(event Collision|EventActorBeginOverlap
  (params (OtherActor :type Actor%20Object%20Reference))
  (bind _enemy1 (Variables|Default|GetEnemy1))
  (bind _returnvalue (Utilities|Select :Index _enemy1 :NewEnumerator0 "/Game/Blueprints/EnemyPawn_Graybeard.EnemyPawn_Graybeard_C" :NewEnumerator1 "/Game/Blueprints/EnemyPawn_Sayaka.EnemyPawn_Sayaka_C" :NewEnumerator2 0))
  (Utilities|Casting|CastToMainCharacterPawn OtherActor)
  (Utilities|FlowControl|DoOnce false
    (:Completed
      (if (Utilities|IsValidClass _returnvalue)
        (bind _returnvalue_2 (AI|SpawnAIFromClass _returnvalue 0 (Transformation|GetWorldLocation (Variables|Default|GetPoint%201)) "0, 0, 0" true 0))
        (if (Utilities|IsValidClass (Utilities|Select :Index (Variables|Default|GetEnemy1) :NewEnumerator0 "/Game/Blueprints/EnemyPawn_Graybeard.EnemyPawn_Graybeard_C" :NewEnumerator1 "/Game/Blueprints/EnemyPawn_Sayaka.EnemyPawn_Sayaka_C" :NewEnumerator2 0))
          (AI|SpawnAIFromClass "/Game/Blueprints/EnemyPawn.EnemyPawn_C" 0 (Transformation|GetWorldLocation (Variables|Default|GetPoint%202)) "0, 0, 0" true 0))))))

(event EventTick
  (params (DeltaSeconds :type Float%20%28single-precision%29)))

(fn ConstructionScript)